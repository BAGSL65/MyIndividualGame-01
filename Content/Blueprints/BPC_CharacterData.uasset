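; BPC_CharacterData is a component Blueprint that holds a character's health and provides functions to change it.
; Add HP raises Health, caps it at MaxHealth and returns the new value.
; Subtract HP lowers Health and reports whether the character will die; a lethal hit returns zero HP without writing it to Health.
; The event graph is unused, so all logic runs through these two calls.
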(fn `Add HP`
  (params (`Added HP` :type "Float (double-precision)"))
  (returns (`After HP` :type "Float (double-precision)"))
  (bind _max_health (`self.Max Health`))
  (bind _returnvalue (+ (`self.Health`) `Added HP`))
  (if (< _returnvalue _max_health)
    (bind _output_get (set `self.Health` _returnvalue))
    (return _output_get)
    (else
      (bind _output_get_2 (set `self.Health` _max_health))
      (return _output_get_2))))

(fn `Subtract HP`
  (params (`Subtract HP` :type "Float (double-precision)"))
  (returns (`WillDie?` :type Boolean) (`After HP` :type "Float (double-precision)"))
  (bind _returnvalue (- (`self.Health`) `Subtract HP`))
  (if (> _returnvalue 0.0)
    (bind _output_get (set `self.Health` _returnvalue))
    (return false _output_get)
    (else
      (return true 0.0))))