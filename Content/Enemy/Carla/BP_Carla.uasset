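; BP_Carla is an enemy that wanders to random reachable points and moves toward the player on sight.
; Patrol loops AIMoveTo with random pauses, continuing only on success, while PawnSensing issues a move toward the player.
; Damage goes through BPCCharacterData to update the WB_Enemy health bar and destroy the actor on death.
; The widget turns toward the player's camera every tick, and UIRadius overlaps toggle its visibility.
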(event `self.ReceiveBeginPlay`
  ;[1 1 1] 初始化
  (bind _asbp_third_person_character (cast `/Game/ThirdPerson/Blueprints/BP_ThirdPersonCharacter` (`GameplayStatics.GetPlayerCharacter` 0)))
  (set `self.PlayerCharacter` _asbp_third_person_character)
  (bind _aswb_enemy (cast `/Game/UI/InGame/WB_Enemy` (`WidgetComponent.GetWidget` (`self.WidgetComponent`))))
  (set `self.UI` _aswb_enemy)
  (`self.Patrol`))

(event `Patrol`
  ;[1 1 1] Patrol
  (`|AIMoveTo` self (`NavigationSystemV1.K2_GetRandomReachablePointInRadius` (`self.K2_GetActorLocation`) 1000.0 null null) null :!label _label
    (:`OnSuccess`
      (`KismetSystemLibrary.PrintString` "Hello")
      (`KismetSystemLibrary.Delay` (`KismetMathLibrary.RandomFloatInRange` 1.0 2.0))
      (goto _label))))

(event `self.ReceiveTick`
  (params (DeltaSeconds :type "Float (single-precision)"))
  (bind _widgetcomponent (`self.WidgetComponent`))
  ;[1 1 1] UI TIck
  (`SceneComponent.K2_SetWorldRotation` _widgetcomponent (`KismetMathLibrary.FindLookAtRotation` (`SceneComponent.K2_GetComponentLocation` _widgetcomponent) (`SceneComponent.K2_GetComponentLocation` (`/Game/ThirdPerson/Blueprints/BP_ThirdPersonCharacter.FollowCamera` (`self.PlayerCharacter`)))) false false))

(event `self.ReceiveAnyDamage`
  (params (Damage :type "Float (single-precision)") (DamageType :type "DamageType Object Reference") (InstigatedBy :type "Controller Object Reference") (DamageCauser :type "Actor Object Reference"))
  (bind _bpc_characterdata (`self.BPC_CharacterData`))
  ;[1 1 1] AnyDamage
  (bind (_willdie_ _after_hp) (`/Game/Blueprints/BPC_CharacterData.Subtract HP` _bpc_characterdata Damage))
  (`ProgressBar.SetPercent` (`/Game/UI/InGame/WB_Enemy.HPBar` (`self.UI`)) (/ _after_hp (`/Game/Blueprints/BPC_CharacterData.Max Health` _bpc_characterdata)))
  (if _willdie_
    (`self.K2_DestroyActor`)))

(event `self.UI radius.OnComponentBeginOverlap`
  (params (OverlappedComponent :type "PrimitiveComponent Object Reference") (OtherActor :type "Actor Object Reference") (OtherComp :type "PrimitiveComponent Object Reference") (OtherBodyIndex :type Integer) (bFromSweep :type Boolean) (SweepResult :type "HitResult Structure (by ref)"))
  ;[1 1 1] Box Collision (UI Visibility)
  (cast `/Game/ThirdPerson/Blueprints/BP_ThirdPersonCharacter` OtherActor)
  (`SceneComponent.SetVisibility` (`self.WidgetComponent`) true false))

(event `self.UI radius.OnComponentEndOverlap`
  (params (OverlappedComponent :type "PrimitiveComponent Object Reference") (OtherActor :type "Actor Object Reference") (OtherComp :type "PrimitiveComponent Object Reference") (OtherBodyIndex :type Integer))
  ;[1 1 1] Box Collision (UI Visibility)
  (cast `/Game/ThirdPerson/Blueprints/BP_ThirdPersonCharacter` OtherActor)
  (`SceneComponent.SetVisibility` (`self.WidgetComponent`) false false))

(event `self.PawnSensing.OnSeePawn`
  (params (Pawn :type "Pawn Object Reference"))
  ;[1 1 1] PawnSensing
  (cast `/Game/ThirdPerson/Blueprints/BP_ThirdPersonCharacter` Pawn)
  (`KismetSystemLibrary.PrintString` "I see You")
  (`|AIMoveTo` self (0.0 0.0 0.0) (`self.PlayerCharacter`) 80.0))

(fn `UserConstructionScript`)